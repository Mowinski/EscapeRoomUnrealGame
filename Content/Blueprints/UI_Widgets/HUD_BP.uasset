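; HUD Blueprint that shows a center-screen dot and battery widget, and manages the pin code entry widget.
; DrawHUD calls AddBatteryWidget, which draws the white dot and creates a new BatteryWidget in the viewport on every draw, with no existing-instance check.
; Events open the stored PinCodeWidget and forward wrong-code feedback to it.
; Closing the pin pad calls RemoveAllWidgets rather than removing only that widget.
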(event `self.ReceiveDrawHUD`
  (params (SizeX :type Integer) (SizeY :type Integer))
  (`self.DrawRect` (struct :`R` 1.0 :`G` 1.0 :`B` 1.0 :`A` 1.0) (`KismetMathLibrary.Conv_IntToDouble` (/ SizeX 2)) (`KismetMathLibrary.Conv_IntToDouble` (/ SizeY 2)) 2.0 2.0)
  (bind _returnvalue (`|CreateWidget` "/Game/Blueprints/UI_Widgets/BatteryWidget.BatteryWidget_C"))
  (`UserWidget.AddToViewport` _returnvalue 0))

(event `Open PinCode Widget`
  (bind _returnvalue (`|CreateWidget` "/Game/Blueprints/UI_Widgets/PinCodeWidget.PinCodeWidget_C"))
  (bind _output_get (set `self.PinCodeWidget` _returnvalue))
  (`UserWidget.AddToViewport` _output_get 0))

(event `Close PinCode Widget`
  (`WidgetLayoutLibrary.RemoveAllWidgets`))

(event `WrongPinCode`
  (`/Game/Blueprints/UI_Widgets/PinCodeWidget.WrongCode` (`self.PinCodeWidget`)))

(fn `UserConstructionScript`)