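; CharacterWithFlashlight is a player character Blueprint that handles basic movement and mouse look.
; Forward and strafe axis inputs feed AddMovementInput along the forward and right vectors of the full control rotation, pitch included.
; Turn and look axis inputs drive controller yaw and pitch directly.
; The construction script is empty, and the graphs contain no flashlight logic despite the asset name.
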(event `InputAxis|Forward_Backward`
  (params (AxisValue :type "Float (single-precision)"))
  ;[1 1 1] Movement
  (`self.AddMovementInput` (`KismetMathLibrary.GetForwardVector` (`self.GetControlRotation`)) AxisValue))

(event `InputAxis|Left_Right`
  (params (AxisValue :type "Float (single-precision)"))
  ;[1 1 1] Movement
  (`self.AddMovementInput` (`KismetMathLibrary.GetRightVector` (`self.GetControlRotation`)) AxisValue))

(event `InputAxis|Rotate_Left_Right`
  (params (AxisValue :type "Float (single-precision)"))
  ;[1 1 1] Mouse movement
  (`self.AddControllerYawInput` AxisValue))

(event `InputAxis|Look_Up_Down`
  (params (AxisValue :type "Float (single-precision)"))
  ;[1 1 1] Mouse movement
  (`self.AddControllerPitchInput` AxisValue))

(fn `UserConstructionScript`)