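; Pin code panel that opens and closes a keypad widget through HUD_BP and checks clicked digits against CorrectCode.
; Each click adds the digit times a growing power of ten, so the first digit is the units, and resets first if Code is already 100 or more.
; A match closes the widget and notifies CharacterWithFlashlight, while a mismatch of 100 or more plays the HUD's wrong-code feedback.
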(event `UsePinCodePanel`
  ;[1 1 1] Show/Hide PinCode Widget
  (bind _ashud_bp (cast `/Game/Blueprints/UI_Widgets/HUD_BP` (`PlayerController.GetHUD` (`GameplayStatics.GetPlayerController` 0))))
  (`/Game/Blueprints/UI_Widgets/HUD_BP.Open PinCode Widget` _ashud_bp))

(event `ReleasePinCodePanel`
  ;[1 1 1] Show/Hide PinCode Widget
  (bind _ashud_bp (cast `/Game/Blueprints/UI_Widgets/HUD_BP` (`PlayerController.GetHUD` (`GameplayStatics.GetPlayerController` 0))))
  (`/Game/Blueprints/UI_Widgets/HUD_BP.Close PinCode Widget` _ashud_bp))

(event `Clicked`
  (params (Digit :type Integer))
  (bind _multipler (`self.Multipler`))
  (bind _correctcode (`self.CorrectCode`))
  (if (>= (`self.Code`) 100)
    (set `self.Code` 0)
    (set `self.Multipler` 1))
  (bind _output_get (set `self.Code` (+ (`self.Code`) (* Digit _multipler))))
  (set `self.Multipler` (* 10 _multipler))
  (if (and (!= _output_get _correctcode) (>= _output_get 100))
    (bind _ashud_bp (cast `/Game/Blueprints/UI_Widgets/HUD_BP` (`PlayerController.GetHUD` (`GameplayStatics.GetPlayerController` 0))))
    (`/Game/Blueprints/UI_Widgets/HUD_BP.WrongPinCode` _ashud_bp)
    (elif (== _output_get _correctcode)
      (bind _ashud_bp_2 (cast `/Game/Blueprints/UI_Widgets/HUD_BP` (`PlayerController.GetHUD` (`GameplayStatics.GetPlayerController` 0))))
      (`/Game/Blueprints/UI_Widgets/HUD_BP.Close PinCode Widget` _ashud_bp_2)
      (bind _ascharacter_with_flashlight (cast `/Game/Blueprints/CharacterWithFlashlight` (`GameplayStatics.GetPlayerPawn` 0)))
      (`/Game/Blueprints/CharacterWithFlashlight.PinCodeCorrect` _ascharacter_with_flashlight))))

(fn `UserConstructionScript`)